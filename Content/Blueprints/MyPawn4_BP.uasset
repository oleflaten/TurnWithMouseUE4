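; MyPawn4_BP is a pawn that turns to face the point under the mouse cursor.
; BeginPlay creates the HUD widget, stores a reference and adds it to the viewport.
; Each tick, a cursor trace against static world objects places the Sphere as a target marker slightly above the hit location.
; The root component then takes its rotation from the height-flattened direction toward that sphere, so aiming stays in the horizontal plane.
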(event EventBeginPlay
  ;[1 1 1] Set up HUD
  (bind _returnvalue (UserInterface|CreateWidget "/Game/Blueprints/HUD.HUD_C"))
  (bind _output_get (Variables|Default|SetHUD_Reference _returnvalue))
  (UserInterface|Viewport|AddtoViewport _output_get 0))

(event EventTick
  (params (DeltaSeconds :type Float%20%28single-precision%29))
  (bind _rootcomponent (Variables|Transformation|GetRootComponent))
  (bind _sphere (Variables|Default|GetSphere))
  (bind _returnvalue (Transformation|GetWorldLocation _rootcomponent))
  (bind _returnvalue_2 (Transformation|GetWorldLocation _sphere))
  ;[1 1 1] Set Target With Mouse
  (Transformation|SetWorldLocation (Variables|Default|GetSphere) (+ (.Location (Collision|BreakHitResult (.HitResult (Class|PlayerController|GetHitResultUnderCursorforObjects (Game|GetPlayerController 0) (Utilities|Array|MakeArray "ObjectTypeQuery1") true)))) "0, 0,30.000000") false false)
  ;[1 1 1] Set Pawn Rotation
  (Transformation|SetWorldRotation _rootcomponent (Math|Conversions|RotationFromXVector (- (Math|Vector|MakeVector (.x _returnvalue_2) (.y _returnvalue_2) 0.0) (Math|Vector|MakeVector (.x _returnvalue) (.y _returnvalue) 0.0))) false false))

(fn ConstructionScript)